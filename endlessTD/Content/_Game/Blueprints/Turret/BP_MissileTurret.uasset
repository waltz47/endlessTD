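; Missile turret actor Blueprint that shows its health through a health bar widget, with any firing behavior not defined in this graph.
; BeginPlay defers to the parent class.
; Every Tick, it casts the widget component's widget to WBP_HealthBar and sets the progress bar to StatComponent's HP divided by MaxHP, polling rather than reacting to damage events.
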(event `self.ReceiveBeginPlay`
  (`parent.ReceiveBeginPlay`))

(event `self.ReceiveTick`
  (params (DeltaSeconds :type "Float (single-precision)"))
  (bind _statcomponent (`self.StatComponent`))
  (bind _returnvalue (`WidgetComponent.GetWidget` (`self.Widget`)))
  (`/Engine/EditorBlueprintResources/StandardMacros.IsValid` _returnvalue
    (:`Is Valid`
      (bind _aswbp_health_bar (cast `/Game/_Game/Blueprints/UI/WBP_HealthBar` _returnvalue))
      (`ProgressBar.SetPercent` (`/Game/_Game/Blueprints/UI/WBP_HealthBar.Progress` _aswbp_health_bar) (/ (`StatComponent.HP` _statcomponent) (`StatComponent.MaxHP` _statcomponent))))))

(fn `UserConstructionScript`)