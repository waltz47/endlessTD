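; Player camera actor for a tower defense game that also holds the build points and handles turret purchases.
; On begin play it shows the cursor, creates the main HUD with itself as player, and starts a looping timer that adds points.
; Tick clamps its X and Y position to fixed map bounds.
; Number keys spend points to spawn gun, missile or multishot turrets, and the Rst action restarts through the game mode.
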(event `self.ReceiveBeginPlay`
  (bind _returnvalue (`GameplayStatics.GetPlayerController` 0))
  (`parent.ReceiveBeginPlay`)
  (set `PlayerController.bShowMouseCursor` true _returnvalue)
  (bind _returnvalue_2 (`|CreateWidget` "/Game/_Game/Blueprints/UI/WBP_MainHUD.WBP_MainHUD_C" _returnvalue self))
  (`UserWidget.AddToViewport` _returnvalue_2 0)
  (`KismetSystemLibrary.K2_SetTimerDelegate` (delegate `ScoringTimer`) 20.0 true 10.0))

(event `ScoringTimer`
  (`/Engine/EditorBlueprintResources/StandardMacros.IncrementInt` (`self.Points`)))

(event `InputAction|Interact`
  (params (Key :type "Key Structure")))

(event `self.ReceiveTick`
  (params (DeltaSeconds :type "Float (single-precision)"))
  (bind _returnvalue_x (`KismetMathLibrary.BreakVector` (`self.K2_GetActorLocation`)))
  (bind (_returnvalue_x_2 _returnvalue_y _returnvalue_z) (`KismetMathLibrary.BreakVector` (`self.K2_GetActorLocation`)))
  (bind (_returnvalue_x_3 _returnvalue_y_2 _returnvalue_z_2) (`KismetMathLibrary.BreakVector` (`self.K2_GetActorLocation`)))
  (bind (_returnvalue_x_4 _returnvalue_y_3 _returnvalue_z_3) (`KismetMathLibrary.BreakVector` (`self.K2_GetActorLocation`)))
  (bind (_returnvalue_x_5 _returnvalue_y_4 _returnvalue_z_4) (`KismetMathLibrary.BreakVector` (`self.K2_GetActorLocation`)))
  (bind (_returnvalue_x_6 _returnvalue_y_5) (`KismetMathLibrary.BreakVector` (`self.K2_GetActorLocation`)))
  (`|ExecutionSequence`
    (:`then_0`
      (`self.K2_SetActorLocation` (`KismetMathLibrary.MakeVector` _returnvalue_x_3 (`KismetMathLibrary.SelectFloat` 6680.0 _returnvalue_y_2 (> _returnvalue_y_2 6680.0)) _returnvalue_z_2)))
    (:`then_1`
      (`self.K2_SetActorLocation` (`KismetMathLibrary.MakeVector` _returnvalue_x_4 (`KismetMathLibrary.SelectFloat` -2620.0 _returnvalue_y_3 (< _returnvalue_y_5 -2620.0)) _returnvalue_z_3)))
    (:`then_2`
      (`self.K2_SetActorLocation` (`KismetMathLibrary.MakeVector` (`KismetMathLibrary.SelectFloat` 4200.0 _returnvalue_x_2 (> _returnvalue_x_2 4200.0)) _returnvalue_y _returnvalue_z)))
    (:`then_3`
      (`self.K2_SetActorLocation` (`KismetMathLibrary.MakeVector` (`KismetMathLibrary.SelectFloat` 100.0 _returnvalue_x_5 (< _returnvalue_x 100.0)) _returnvalue_y_4 _returnvalue_z_4)))))

(event `Key|One`
  (params (Key :type "Key Structure"))
  (:`Pressed`
    (if (>= (`self.Points`) 3)
      (`|SpawnActorFromClass` "/Game/_Game/Blueprints/Turret/BP_GunTurret.BP_GunTurret_C" (`KismetMathLibrary.MakeTransform` (0.0 0.0 0.0)) "Undefined" "OverrideRootScale" null null)
      (set `self.Points` (- (`self.Points`) 3)))))

(event `Key|Two`
  (params (Key :type "Key Structure"))
  (:`Pressed`
    (if (>= (`self.Points`) 5)
      (`|SpawnActorFromClass` "/Game/_Game/Blueprints/Turret/BP_MissileTurret.BP_MissileTurret_C" (`KismetMathLibrary.MakeTransform` (0.0 0.0 0.0)) "Undefined" "OverrideRootScale" null null)
      (set `self.Points` (- (`self.Points`) 5)))))

(event `Key|Three`
  (params (Key :type "Key Structure"))
  (:`Pressed`
    (if (>= (`self.Points`) 20)
      (`|SpawnActorFromClass` "/Game/_Game/Blueprints/Turret/BP_MultishotTurret.BP_MultishotTurret_C" (`KismetMathLibrary.MakeTransform` (0.0 0.0 0.0)) "Undefined" "OverrideRootScale" null null)
      (set `self.Points` (- (`self.Points`) 20)))))

(event `InputAction|Rst`
  (params (Key :type "Key Structure"))
  (:`Pressed`
    (bind _asbp_tdgame_mode_not_base (cast `/Game/_Game/Blueprints/BP_TDGameModeNotBase` (`GameplayStatics.GetGameMode`)))
    (`GameMode.RestartGame` _asbp_tdgame_mode_not_base)))

(fn `UserConstructionScript`)