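; BP_GridManager throttles enemy spawning and spawns nukes on double-clicked grid tiles.
; On BeginPlay it caches all enemy spawners and starts a looping timer that toggles their Active flag by whether the live Enemy count exceeds a fixed cap.
; DoubleClickedTile spawns a BP_Nuke high above the clicked GridTile, passes that tile as its target and activates it.
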(event `self.ReceiveBeginPlay`
  (bind _outactors (`GameplayStatics.GetAllActorsOfClass` "/Game/_Game/Blueprints/WorldActors/Spawner/BP_EnemySpawner.BP_EnemySpawner_C"))
  (set `self.Out Actors` _outactors)
  (`KismetSystemLibrary.K2_SetTimerDelegate` (delegate `AiCheck`) 10.0 true 15.0))

(event `AiCheck`
  (bind _outactors (`GameplayStatics.GetAllActorsOfClass` "/Script/endlessTD.Enemy"))
  (if (> (`KismetArrayLibrary.Array_Length` _outactors) 80)
    (for _array_element (`self.Out Actors`)
      (set `EnemySpawner.Active` false _array_element))
    (else
      (for _array_element_2 (`self.Out Actors`)
        (set `EnemySpawner.Active` true _array_element_2)))))

(event `self.DoubleClickedTile`
  (params (Actor :type "Actor Object Reference"))
  (bind (_returnvalue_x _returnvalue_y) (`KismetMathLibrary.BreakVector` (`self.K2_GetActorLocation` Actor)))
  (`/Engine/EditorBlueprintResources/StandardMacros.IsValid` Actor
    (:`Is Valid`
      (bind _asgrid_tile (cast `GridTile` Actor))
      (bind _returnvalue (`|SpawnActorFromClass` "/Game/_Game/Blueprints/WorldActors/Nuke/BP_Nuke.BP_Nuke_C" (`KismetMathLibrary.MakeTransform` (`KismetMathLibrary.MakeVector` _returnvalue_x _returnvalue_y 5000.0)) "Undefined" "OverrideRootScale" null _asgrid_tile null))
      (`/Engine/EditorBlueprintResources/StandardMacros.IsValid` _returnvalue
        (:`Is Valid`
          (`/Game/_Game/Blueprints/WorldActors/Nuke/BP_Nuke.Activate` _returnvalue))))))

(fn `UserConstructionScript`)