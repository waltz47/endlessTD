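; BP_Nuke is a projectile actor that explodes on its first overlap, wiping out nearby enemies and grid tile occupants.
; Activate arms it if TargetTile is valid, setting a homing target but leaving homing off; otherwise it destroys itself.
; A radius query destroys victims, while the nuke removes itself only upon finding an AttackTag actor.
; The target tile gets marked destroyed and turned red, with a camera shake.
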(event `self.ReceiveBeginPlay`
  (`self.Activate`))

(event `self.Sphere.OnComponentBeginOverlap`
  (params (OverlappedComponent :type "PrimitiveComponent Object Reference") (OtherActor :type "Actor Object Reference") (OtherComp :type "PrimitiveComponent Object Reference") (OtherBodyIndex :type Integer) (bFromSweep :type Boolean) (SweepResult :type "HitResult Structure (by ref)"))
  (if (`self.Active`)
    (`/Engine/EditorBlueprintResources/StandardMacros.IsValid` self
      (:`Is Valid`
        (`/Engine/EditorBlueprintResources/StandardMacros.IsValid` OtherActor
          (:`Is Valid`
            (if (!= OtherActor self)
              (set `self.Active` false)
              (`GameplayStatics.SpawnEmitterAtLocation` "/Game/M5VFXVOL2/Particles/Explosion/Fire_Exp_00.Fire_Exp_00" (`self.K2_GetActorLocation`) (struct) (5.0 5.0 5.0) true "AutoRelease")
              (bind _outactors (`KismetSystemLibrary.SphereOverlapActors` (`self.K2_GetActorLocation`) (`self.CoverRadius`) (`|MakeArray` "ObjectTypeQuery3" "ObjectTypeQuery2" "ObjectTypeQuery1" "ObjectTypeQuery4" :!type "EObjectTypeQuery Enum") "/Script/Engine.Actor"))
              (for _array_element _outactors
                (`/Engine/EditorBlueprintResources/StandardMacros.IsValid` self
                  (:`Is Valid`
                    (bind _asenemy (cast `Enemy` _array_element)
                      (:`then`
                        (`self.K2_DestroyActor` _asenemy))
                      (:`CastFailed`
                        (bind _asbp_grid_tile (cast `/Game/_Game/Blueprints/Grid/BP_GridTile` _array_element)
                          (:`then`
                            (bind _occupied (`GridTile.Occupied` _asbp_grid_tile)
                              (:`then`
                                (`self.K2_DestroyActor` _occupied))
                              (:`else`)))
                          (:`CastFailed`
                            (if (`self.ActorHasTag` _array_element "AttackTag")
                              (`self.K2_DestroyActor`)))))))))
              (bind _targettile (`self.TargetTile`)
                (:`then`
                  (set `GridTile.Destroyed` true _targettile)
                  (`PrimitiveComponent.SetMaterial` (`GridTile.TileMesh` _targettile) 0 "/Game/_Game/Materials/MAT_Red.MAT_Red")
                  (`GameplayStatics.PlayWorldCameraShake` "/Game/_Game/Blueprints/WorldActors/Nuke/BP_WorldShake2.BP_WorldShake2_C" (`self.K2_GetActorLocation` _targettile) 10.0 5000.0 0.5))
                (:`else`)))))))))

(fn `Activate`
  (bind _projectilemovement (`self.ProjectileMovement`))
  (bind _targettile (`self.TargetTile`)
    (:`then`
      (set `ProjectileMovementComponent.HomingTargetComponent` (`GridTile.SceneRoot` _targettile) _projectilemovement)
      (set `ProjectileMovementComponent.bIsHomingProjectile` false _projectilemovement)
      (set `self.Active` true))
    (:`else`
      (`self.K2_DestroyActor`))))

(fn `UserConstructionScript`)