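; BP_Zombie is a melee enemy character that attacks the target stored in its AI blackboard.
; MeleeAttack plays the attack montage, locked by a CanAttack flag until it completes or is interrupted.
; Handlemeleedamage checks the sphere's overlapping actors and applies StatComponent damage to the one tagged AttackTag that matches TargetActor.
; The construction script randomizes max walk speed so zombies move at varied paces.
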(event `self.ReceiveBeginPlay`
  (`parent.ReceiveBeginPlay`))

(event `Handlemeleedamage`
  (for _array_element (`PrimitiveComponent.GetOverlappingActors` (`self.Sphere`) "/Script/Engine.Actor")
    (if (`self.ActorHasTag` _array_element "AttackTag")
      (bind _asactor (cast `Actor` (`BlackboardComponent.GetValueAsObject` (`AIBlueprintHelperLibrary.GetBlackboard` self) (`KismetStringLibrary.Conv_StringToName` "TargetActor"))))
      (if (== _array_element _asactor)
        (bind _returnvalue (`StatComponent.GetDamage` (`self.StatComponent`)))
        (`GameplayStatics.ApplyDamage` _asactor _returnvalue)))))

(event `MeleeAttack`
  (if (`self.canAttack`)
    (set `self.canAttack` false)
    (`|PlayMontage` (`self.Mesh`) (`self.AttackMontage`)
      (:`OnCompleted`
        _)
      (:`OnInterrupted`
        _))
    (set `self.canAttack` true)))

(fn `UserConstructionScript`
  (`parent.UserConstructionScript`)
  (set `CharacterMovementComponent.MaxWalkSpeed` (`KismetMathLibrary.RandomFloatInRange` 350.0 500.0) (`self.CharacterMovement`)))